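; CarBP is a car that drives along the spline of a randomly chosen RouteBP and destroys itself at the end.
; A timeline drives position and rotation, starting at SpawnPoint (randomly delayed when zero), with play rate scaled by spline length for consistent speed.
; Overlap with Orangutaun_BP enables cube physics, launches it sideways and stops the timeline, then destroys the car and spawns a replacement after a delay.
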(event `self.ReceiveBeginPlay`
  ;[1 1 1] Where to add randomness
  (bind _outactors (`GameplayStatics.GetAllActorsOfClass` "/Game/Characters/Cars/SplinePaths/RouteBP.RouteBP_C"))
  (set `self.RouteRef` (`|GetArrayItem` _outactors (`KismetMathLibrary.RandomInteger` (`KismetArrayLibrary.Array_Length` _outactors))))
  (`TimelineComponent.SetPlaybackPosition` (`self.Move Car Timeline`) (`self.SpawnPoint`) false true)
  (if (not (!= (`self.SpawnPoint`) 0.0))
    (`KismetSystemLibrary.Delay` (`KismetMathLibrary.RandomFloatInRange` 0.0 4.0)))
  (`self.Move Car`)
  (`KismetSystemLibrary.PrintString` (`KismetStringLibrary.Conv_DoubleToString` (`SplineComponent.GetSplineLength` (`/Game/Characters/Cars/SplinePaths/RouteBP.Spline` (`self.RouteRef`))))))

(event `Move Car`
  (bind _spline (`/Game/Characters/Cars/SplinePaths/RouteBP.Spline` (`self.RouteRef`)))
  (`TimelineComponent.SetPlayRate` (`self.Move Car Timeline`) (/ 1.0 (/ (`SplineComponent.GetSplineLength` (`/Game/Characters/Cars/SplinePaths/RouteBP.Spline` (`self.RouteRef`))) 1000.0)))
  (bind (_direction _move_track) (`Timeline|Move Car Timeline` :!label _label)
    (:`Update`
      (bind _returnvalue (`KismetMathLibrary.Lerp` 0.0 (`SplineComponent.GetSplineLength` _spline) _move_track))
      (`self.K2_SetActorTransform` (`KismetMathLibrary.MakeTransform` (`SplineComponent.GetLocationAtDistanceAlongSpline` _spline _returnvalue "World") (`SplineComponent.GetRotationAtDistanceAlongSpline` _spline _returnvalue "Local"))))
    (:`Finished`
      (`self.K2_DestroyActor`))))

(event `self.Box.OnComponentBeginOverlap`
  (params (OverlappedComponent :type "PrimitiveComponent Object Reference") (OtherActor :type "Actor Object Reference") (OtherComp :type "PrimitiveComponent Object Reference") (OtherBodyIndex :type Integer) (bFromSweep :type Boolean) (SweepResult :type "HitResult Structure (by ref)"))
  (bind _cube (`self.Cube`))
  (bind _asorangutaun_bp (cast `/Game/Characters/Oranguton/Blueprints/Orangutaun_BP` OtherActor))
  (`PrimitiveComponent.SetSimulatePhysics` (`self.Cube`) true)
  (if (`KismetSystemLibrary.IsValid` _cube)
    (`PrimitiveComponent.AddImpulse` _cube (* (`SceneComponent.GetRightVector` (`Character.Mesh` _asorangutaun_bp)) 20000.0) "None" false)
    (`|ExecutionSequence`
      (:`then_0`
        (goto _label :!via `Stop`))
      (:`then_1`
        (`KismetSystemLibrary.Delay` 5.0)
        (if (`KismetSystemLibrary.IsValid` self)
          (`self.K2_DestroyActor`)
          (`|SpawnActorFromClass` "CarBP_C" (`KismetMathLibrary.MakeTransform` (0.0 0.0 0.0)) "Undefined" "OverrideRootScale" null null))))))

(fn `UserConstructionScript`)