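; Human NPC that flees from the player-type Orangutaun character and dies when touched by it.
; Pawn sensing stores a seen Orangutaun and starts RunAway, which uses AI MoveTo toward a point 1000 units directly away at the human's current height.
; Each successful move restarts the flight, with no handling for failed moves.
; Box overlap with an Orangutaun increments that character's KillCount and destroys the human.
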(event `self.PawnSensing.OnSeePawn`
  (params (Pawn :type "Pawn Object Reference"))
  (bind _asorangutaun_bp (cast `/Game/Characters/Oranguton/Blueprints/Orangutaun_BP` Pawn))
  (`KismetSystemLibrary.PrintString` "Yoikes")
  (set `self.Orangutaun` _asorangutaun_bp)
  (`self.RunAway`))

(event `RunAway`
  (bind _returnvalue (`self.K2_GetActorLocation`))
  (`|AIMoveTo` self (`KismetMathLibrary.MakeVector` (.x (+ _returnvalue (* (`KismetMathLibrary.GetForwardVector` (`KismetMathLibrary.FindLookAtRotation` _returnvalue (`self.K2_GetActorLocation` (`self.Orangutaun`)))) -1000.0))) (.y (+ _returnvalue (* (`KismetMathLibrary.GetForwardVector` (`KismetMathLibrary.FindLookAtRotation` _returnvalue (`self.K2_GetActorLocation` (`self.Orangutaun`)))) -1000.0))) (.z _returnvalue)) null
    (:`OnSuccess`
      (`KismetSystemLibrary.PrintString` "safe")
      (`self.RunAway`))))

(event `self.Box.OnComponentBeginOverlap`
  (params (OverlappedComponent :type "PrimitiveComponent Object Reference") (OtherActor :type "Actor Object Reference") (OtherComp :type "PrimitiveComponent Object Reference") (OtherBodyIndex :type Integer) (bFromSweep :type Boolean) (SweepResult :type "HitResult Structure (by ref)"))
  (bind _asorangutaun_bp (cast `/Game/Characters/Oranguton/Blueprints/Orangutaun_BP` OtherActor))
  (`/Engine/EditorBlueprintResources/StandardMacros.IncrementInt` (`/Game/Characters/Oranguton/Blueprints/Orangutaun_BP.KillCount` _asorangutaun_bp)
    (:`  `
      (`self.K2_DestroyActor`))))

(fn `UserConstructionScript`)